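; BP_Generator is a repairable generator that tracks its repair progress as a value clamped between zero and RepairValue.
; Repair adds progress and plays a success sound with a message when full, while Bomb removes a fixed amount, plays a blast sound and triggers a shake.
; The shake is a timeline that rocks BodyRoot on its roll axis.
; GetRepairPercent and IsRepaired expose the progress ratio and completion state.
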(event Custom|Bomb
  ;[1 1 1] Bomb
  (Variables|Default|SetcurrentRepairValue (Math|Float|Clamp(Float) (- (Variables|Default|GetcurrentRepairValue) 1e+01) 0.0 (Variables|Default|GetrepairValue)))
  (Development|PrintString "Bomb" true true "(R=1.000000,G=0.010379,B=0.000000,A=1.000000)")
  (CallFunction|StartShake)
  (Audio|PlaySound2D "/Game/Sounds/Bomb.Bomb" 0.5 1.0 0.0 0 0))

(event Custom|Repair
  (params (value :type Float%20%28single-precision%29))
  ;[1 1 1] Repair
  (Variables|Default|SetcurrentRepairValue (Math|Float|Clamp(Float) (+ (Variables|Default|GetcurrentRepairValue) value) 0.0 (Variables|Default|GetrepairValue)))
  (if (CallFunction|IsRepaired)
    (Audio|PlaySound2D "/Engine/EditorSounds/Notifications/CompileSuccess.CompileSuccess" 1.0 1.0 0.0 0 0)
    (Development|PrintString "RepairSuccess" true true "(R=1.000000,G=0.329981,B=0.000000,A=1.000000)")))

(event Custom|StartShake
  (bind _returnvalue (Math|Float|MakeLiteralFloat 3e+01))
  ;[1 1 1] StartShake
  (bind _alpha (Timeline|TL_Shake PlayFromStart)
    (:Update
      (Transformation|SetRelativeRotation (Variables|Default|GetBodyRoot) (Math|Rotator|Lerp(Rotator) (Math|Rotator|MakeRotator (* _returnvalue -1.0) 0.0 0.0) (Math|Rotator|MakeRotator _returnvalue 0.0 0.0) (Math|Float|MapRangeClamped _alpha -1.0 1.0 0.0 1.0)) false false))))

(fn ConstructionScript)

(fn GetRepairPercent
  (return (/ (Variables|Default|GetcurrentRepairValue) (Variables|Default|GetrepairValue))))

(fn IsRepaired
  (return (== (Variables|Default|GetrepairValue) (Variables|Default|GetcurrentRepairValue))))